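; BP_StairwayToHeaven_GI, by its name the game instance, manages a single 2D music track.
; StartMusic creates and plays a sound at half volume only when none is stored, with caller-set options for level-transition persistence and auto-destroy.
; StopMusic stops the stored sound and clears the reference, allowing another track to start.
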(fn `StartMusic`
  (params (Audio :type "SoundBase Object Reference") (bPersistAcrossLevelTransition :type Boolean) (bAutoDestroy :type Boolean))
  (if (not (`KismetSystemLibrary.IsValid` (`self.SoundPlaying`)))
    (bind _returnvalue (`GameplayStatics.CreateSound2D` Audio 0.5 1.0 0.0 null bPersistAcrossLevelTransition bAutoDestroy))
    (bind _output_get (set `self.SoundPlaying` _returnvalue))
    (`AudioComponent.Play` _output_get 0.0)))

(fn `StopMusic`
  (if (`KismetSystemLibrary.IsValid` (`self.SoundPlaying`))
    (`AudioComponent.Stop` (`self.SoundPlaying`))
    (set `self.SoundPlaying` null)))